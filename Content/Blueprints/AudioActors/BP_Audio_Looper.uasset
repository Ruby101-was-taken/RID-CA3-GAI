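; BP_Audio_Looper is an audio actor that repeatedly plays a sound at its audio component's location at random intervals.
; The construction script copies the exposed sound, volume, pitch and attenuation settings onto the component.
; Tick drives a random Delay between LoopMin and LoopMax, then fires PlaySoundAtLocation.
; That call takes only the component's sound and location, not its volume, pitch or attenuation.
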(event EventTick
  (params (DeltaSeconds :type Float%20%28single-precision%29))
  (bind _audiocomponent (Variables|Default|GetAudioComponent))
  ;[0.15 0.15 0.15 0.5] Set Random Delay
  (Utilities|FlowControl|Delay (Math|Random|RandomFloatinRange (Variables|SoundConfig|Getloop_min) (Variables|SoundConfig|Getloop_max)))
  ;[0.15 0.15 0.15 0.5] Play the Sound
  (Audio|PlaySoundatLocation (Variables|/Script/Engine.AudioComponent|GetSound _audiocomponent) (Transformation|GetWorldLocation _audiocomponent) "0, 0, 0" 1.0 1.0 0.0 0 0 0 0))

(fn ConstructionScript
  (bind _audiocomponent (Variables|Default|GetAudioComponent))
  ;[0.15 0.15 0.15 0.5] Set Sound Settings
  (Audio|Components|Audio|SetSound _audiocomponent (Variables|SoundConfig|Getsound))
  (Audio|Components|Audio|SetVolumeMultiplier _audiocomponent (Variables|SoundConfig|Getvolume_multiplier) :!class /Script/Engine.AudioComponent)
  (Audio|Components|Audio|SetPitchMultiplier _audiocomponent (Variables|SoundConfig|Getpitch_multiplier))
  (Variables|/Script/Engine.AudioComponent|SetAttenuationSettings _audiocomponent (Variables|AttenuationConfig|Getattenuation_settings)))