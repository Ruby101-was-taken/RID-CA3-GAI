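; BP_Pillar is a pillar actor that moves vertically by UpwardDistance from the location it records at BeginPlay.
; Move triggers ExecuteMove and prints a debug message.
; ExecuteMove plays MovementTimeline from the start, scaling its play rate by the inverse of MoveDuration, and lerps the actor location along Z without sweeping.
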(event Custom|ExecuteMove
  (bind _startlocation (Variables|Config|GetStartLocation))
  ;[0.15 0.15 0.15 0.5] Set Play Rate
  (Components|Timeline|SetPlayRate (Variables|Default|GetMovementTimeline) (/ 1.0 (Variables|Config|GetMoveDuration)))
  (bind _alpha (Timeline|MovementTimeline PlayFromStart)
    (:Update
      (Transformation|SetActorLocation (Math|Vector|Lerp(Vector) _startlocation (+ _startlocation (Math|Vector|MakeVector 0.0 0.0 (Variables|Config|GetUpwardDistance))) _alpha) false false))))

(event EventBeginPlay
  (Variables|Config|SetStartLocation (Transformation|GetActorLocation)))

(fn ConstructionScript)

(fn Move
  (CallFunction|ExecuteMove)
  (Development|PrintString "Execute Move!"))