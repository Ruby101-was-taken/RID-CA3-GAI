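; Camp deposit station that collects bugs and opens the world's gates once enough are deposited.
; AddBug appends to the Bugs array and, when the count reaches exactly two, finds every BP_Gate actor and calls Open on each.
; ShowAllBugs prints the stored bugs' names, and the event graph holds no active logic, so both functions rely on outside callers.
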(event EventBeginPlay)

(event Collision|EventActorBeginOverlap
  (params (OtherActor :type Actor%20Object%20Reference)))

(event EventTick
  (params (DeltaSeconds :type Float%20%28single-precision%29)))

(fn ConstructionScript)

(fn AddBug
  (params (bug :type S%20Bug%20Info%20Structure))
  (bind _bugs (Variables|Default|Getbugs))
  (Utilities|Array|Add _bugs bug)
  (if (== (Utilities|Array|Length _bugs) 2)
    (bind _outactors (Actor|GetAllActorsOfClass "/Game/Blueprints/World/Interractables/Camp/BP_Gate.BP_Gate_C"))
    (for _array_element _outactors
      (Default|Open _array_element))))

(fn ShowAllBugs
  (for _array_element (Variables|Default|Getbugs)
    (Development|PrintString (.name _array_element))))