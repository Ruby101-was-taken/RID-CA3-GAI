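; BP_Gate is a camp gate actor that swings open by itself a few seconds after play begins.
; BeginPlay waits on a delay, then calls Open, which sets the ShouldBeOpen flag.
; While the flag is set, Tick eases the Pivot component's yaw toward a fixed open angle by lerping from its current value with DeltaSeconds as alpha.
; It has no closing logic.
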(event EventBeginPlay
  (Utilities|FlowControl|Delay 4.0)
  (CallFunction|Open))

(event Collision|EventActorBeginOverlap
  (params (OtherActor :type Actor%20Object%20Reference)))

(event EventTick
  (params (DeltaSeconds :type Float%20%28single-precision%29))
  (bind _pivot (Variables|Default|GetPivot))
  (bind _relativerotation (Variables|/Script/Engine.SceneComponent|GetRelativeRotation _pivot))
  (if (Variables|Default|Getshould_be_open)
    (Transformation|SetRelativeLocationAndRotation _pivot (Variables|/Script/Engine.SceneComponent|GetRelativeLocation _pivot) (Math|Rotator|MakeRotator (.roll _relativerotation) (.pitch _relativerotation) (Math|Float|Lerp (.yaw _relativerotation) 56.0 DeltaSeconds)) false false)))

(fn ConstructionScript)

(fn Open
  (Variables|Default|Setshould_be_open true))